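; PacingEnnemi_BP is an enemy that paces back and forth between its spawn point and a target actor.
; On BeginPlay it records its spawn location, then uses AIMoveTo toward the first BP_Target found in the level.
; After success or failure of each move it waits briefly and heads the other way, looping MoveToTarget and Return indefinitely.
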(event Custom|MoveToTarget
  (bind _outactors (Actor|GetAllActorsOfClass "/Game/BP_Target.BP_Target_C"))
  (AI|AIMoveTo self "0, 0, 0" (Utilities|Array|Get(acopy) _outactors) 5.0 false
    (:OnSuccess
      _)
    (:OnFail
      _))
  (Utilities|FlowControl|Delay 1.0)
  (CallFunction|Return))

(event Custom|Return
  (AI|AIMoveTo self (Variables|Default|GetSpawningLocation) 0 5.0 false
    (:OnSuccess
      _)
    (:OnFail
      _))
  (Utilities|FlowControl|Delay 1.0)
  (CallFunction|MovetoTarget))

(event EventBeginPlay
  (Variables|Default|SetSpawningLocation (Transformation|GetActorLocation))
  (CallFunction|MovetoTarget))

(fn ConstructionScript)