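; Player-controlled hero character with Enhanced Input movement and look, plus a simple health and respawn system.
; BeginPlay adds the hero mapping context and puts the hero widget on screen.
; Movement follows the control rotation, and look input drives controller yaw and pitch.
; Damage lowers clamped health; at zero the hero teleports to a hardcoded location and health refills, without being destroyed.
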(event Input|EnhancedActionEvents|EnhancedInputActionHeroMouvement_IA
  (params (ActionValue :type Vector%202D%20Structure) (ElapsedSeconds :type Float%20%28double-precision%29) (TriggeredSeconds :type Float%20%28double-precision%29) (InputAction :type Input%20Action%20Object%20Reference :default "/Game/HeroMouvement_IA.HeroMouvement_IA"))
  (bind _returnvalue (Pawn|GetControlRotation :!class /Script/Engine.Pawn))
  (Pawn|Input|AddMovementInput (Math|Vector|GetForwardVector (Math|Rotator|MakeRotator 0.0 0.0 (.yaw (Pawn|GetControlRotation :!class /Script/Engine.Pawn)))) (.y ActionValue) false)
  (Pawn|Input|AddMovementInput (Math|Vector|GetRightVector (Math|Rotator|MakeRotator (.roll _returnvalue) 0.0 (.yaw _returnvalue))) (.x ActionValue) false))

(event Input|EnhancedActionEvents|EnhancedInputActionHeroLook_IA
  (params (ActionValue :type Vector%202D%20Structure) (ElapsedSeconds :type Float%20%28double-precision%29) (TriggeredSeconds :type Float%20%28double-precision%29) (InputAction :type Input%20Action%20Object%20Reference :default "/Game/HeroLook_IA.HeroLook_IA"))
  (Pawn|Input|AddControllerYawInput (.x ActionValue))
  (Pawn|Input|AddControllerPitchInput (.y ActionValue)))

(event Game|Damage|EventAnyDamage
  (params (Damage :type Float%20%28single-precision%29) (DamageType :type Damage%20Type%20Object%20Reference) (InstigatedBy :type Controller%20Object%20Reference) (DamageCauser :type Actor%20Object%20Reference))
  (bind _output_get (Variables|Default|SetCurrentHealth (Math|Float|Clamp(Float) (- (Variables|Default|GetCurrentHealth) Damage) 0.0 (Variables|Default|GetTotalHealth))))
  (if (== _output_get 0.0)
    (Transformation|SetActorTransform (Math|Transform|MakeTransform "887.417534,-3209.412364,92.000000" "0, 0, 0" "1.000000,1.000000,1.000000") false true)
    (Variables|Default|SetCurrentHealth (Variables|Default|GetTotalHealth))))

(event EventBeginPlay
  (bind _returnvalue (Game|GetPlayerController 0))
  (bind _returnvalue_2 (PlayerController|LocalPlayerSubsystems|GetEnhancedInputLocalPlayerSubsystem _returnvalue))
  (Utilities|IsValid _returnvalue_2
    (:Is%20Valid
      (Input|AddMappingContext _returnvalue_2 "/Game/Hero_IMC.Hero_IMC" 0 "(bIgnoreAllPressedKeysUntilRelease=True,bForceImmediately=False,bNotifyUserSettings=False)")
      (bind _returnvalue_3 (UserInterface|CreateWidget "/Game/HeroWidget_BP.HeroWidget_BP_C"))
      (UserInterface|Viewport|AddtoViewport _returnvalue_3 0))))

(fn ConstructionScript)