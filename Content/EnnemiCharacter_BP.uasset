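; Enemy character Blueprint that wanders the navmesh at random and chases pawns it sees.
; It loops AI moves to random nearby points, pausing a random delay after each success or failure.
; When PawnSensing sees a pawn, it raises walk speed and moves toward it, restoring slower speed once that move ends.
; Capsule hits apply fixed damage to whatever actor it bumps, without filtering.
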(event OnSeePawn(PawnSensing)
  (params (Pawn :type Pawn%20Object%20Reference))
  (bind _charactermovement (Variables|Character|GetCharacterMovement))
  (Variables|/Script/Engine.CharacterMovementComponent|SetMaxWalkSpeed _charactermovement 1e+03)
  (AI|AIMoveTo self "0, 0, 0" Pawn 5.0 false
    (:OnSuccess
      _)
    (:OnFail
      _))
  (Variables|/Script/Engine.CharacterMovementComponent|SetMaxWalkSpeed _charactermovement 3e+02))

(event OnComponentHit(CapsuleComponent)
  (params (HitComponent :type Primitive%20Component%20Object%20Reference) (OtherActor :type Actor%20Object%20Reference) (OtherComp :type Primitive%20Component%20Object%20Reference) (NormalImpulse :type Vector :default "0, 0, 0") (Hit :type Hit%20Result%20Structure%20%28by%20ref%29))
  (Game|Damage|ApplyDamage OtherActor 5e+01 0 self))

(event Custom|MoveToRandomLocation
  (bind _randomlocation (Class|NavigationSystemV1|GetRandomLocationinNavigableRadius (Transformation|GetActorLocation) 1e+03 0 0))
  (AI|AIMoveTo self _randomlocation 0 5.0 false
    (:OnSuccess
      _)
    (:OnFail
      _))
  (Utilities|FlowControl|Delay (* (Math|Random|RandomFloat) 1e+01))
  (CallFunction|MovetoRandomLocation))

(event EventBeginPlay
  (CallFunction|MovetoRandomLocation))

(fn ConstructionScript)